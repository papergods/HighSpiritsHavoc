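; Laser card that fires a hitscan beam from the character along the camera's forward direction when used.
; Its UseCard override runs a Visibility line trace out to LaserDistance, with persistent debug drawing left on.
; On a hit it spawns a fire effect at the impact point and calls the parent UseCard; a miss skips both.
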(event EventBeginPlay)

(event Collision|EventActorBeginOverlap
  (params (OtherActor :type Actor%20Object%20Reference)))

(event EventTick
  (params (DeltaSeconds :type Float%20%28single-precision%29)))

(fn ConstructionScript
  (|CallParentFunction))

(fn UseCard
  (params (SpawnLocationBullet :type Vector :default "0, 0, 0") (SpawnLocationCharacter :type Vector :default "0, 0, 0") (SpawnLocationFargroundBlast :type Vector :default "0, 0, 0") (CameraRotation :type Rotator :default "0, 0, 0"))
  (bind (_outhit _returnvalue) (Collision|LineTraceByChannel SpawnLocationCharacter (+ (* (Math|Vector|GetForwardVector CameraRotation) (Variables|Default|GetLaserDistance)) SpawnLocationCharacter) "TraceTypeQuery1" false 0 "Persistent"))
  (if _returnvalue
    (Game|SpawnActorfromClass "/Game/StarterContent/Blueprints/Blueprint_Effect_Fire.Blueprint_Effect_Fire_C" (Math|Conversions|ToTransform(Vector) (.Location (Collision|BreakHitResult _outhit))) "Undefined" 0 0)
    (bind _spiritcost (|CallParentFunction "0, 0, 0" "0, 0, 0" "0, 0, 0" "0, 0, 0"))
    (return _spiritcost)))